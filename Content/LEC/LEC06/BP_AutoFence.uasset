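; BP_AutoFence is a procedural fence actor that builds a straight row of static mesh pieces from its origin toward FenceEnd.
; The construction script derives the count from the vector's length and adds a component every 20 units along its direction.
; Each piece faces along the fence with slight random yaw and height scale, which re-roll whenever construction reruns.
; The event graph holds no logic.
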(event EventBeginPlay)

(event Collision|EventActorBeginOverlap
  (params (OtherActor :type Actor%20Object%20Reference)))

(event EventTick
  (params (DeltaSeconds :type Float%20%28single-precision%29)))

(fn ConstructionScript
  (bind _fenceend (Variables|Default|GetFenceEnd))
  (Variables|Default|SetUnitDirextion (Math|Vector|Normalize _fenceend))
  (for _index (range 0 (Math|Float|Truncate (/ (Math|Vector|VectorLength _fenceend) 2e+01)))
    (AddComponent|AddStaticMeshComponent false (Math|Transform|MakeTransform (* _index 20 (Variables|Default|GetUnitDirextion)) (Math|Rotator|CombineRotators (Math|Conversions|RotationFromXVector (Variables|Default|GetUnitDirextion)) (Math|Rotator|MakeRotator 0.0 0.0 (Math|Random|RandomFloatinRange -8.0 8.0))) (Math|Vector|MakeVector 1.0 1.0 (Math|Random|RandomFloatinRange 0.98 1.02))))))