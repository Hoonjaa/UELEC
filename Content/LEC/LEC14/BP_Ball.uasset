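; BP_Ball is a projectile ball that damages whatever it hits.
; On BeginPlay it feeds InitialVelocity into its ProjectileMovement component, activates it, and enables mesh collision after a short delay.
; When the mesh registers a hit, it applies fixed damage to the other actor and switches on physics simulation for the ball.
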(event OnComponentHit(StaticMeshComponent)
  (params (HitComponent :type Primitive%20Component%20Object%20Reference) (OtherActor :type Actor%20Object%20Reference) (OtherComp :type Primitive%20Component%20Object%20Reference) (NormalImpulse :type Vector :default "0, 0, 0") (Hit :type Hit%20Result%20Structure%20%28by%20ref%29))
  (Game|Damage|ApplyDamage OtherActor 2e+01 0 0)
  (Physics|SetSimulatePhysics (Variables|Debug|GetStaticMeshComponent) true))

(event EventBeginPlay
  (bind _projectilemovement (Variables|Default|GetProjectileMovement))
  (Variables|/Script/Engine.MovementComponent|SetVelocity _projectilemovement (Variables|Default|GetInitialVelocity))
  (Components|Activation|Activate _projectilemovement false)
  (Utilities|FlowControl|Delay 0.1)
  (Collision|SetCollisionEnabled (Variables|Debug|GetStaticMeshComponent) "QueryAndPhysics"))

(event Collision|EventActorBeginOverlap
  (params (OtherActor :type Actor%20Object%20Reference)))

(event EventTick
  (params (DeltaSeconds :type Float%20%28single-precision%29)))

(fn ConstructionScript)