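; BP_Course builds a randomized course for the AircraftRacing practice game along the vector to End.
; The construction script adds a static mesh every 10,000 units along that line, randomly offset in local Y and Z.
; Each point has a random chance to also get a child actor at the same relative location.
; Randomness is unseeded, so the layout re-rolls whenever construction reruns; the event graph has no runtime logic.
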(event EventBeginPlay)

(event Collision|EventActorBeginOverlap
  (params (OtherActor :type Actor%20Object%20Reference)))

(event EventTick
  (params (DeltaSeconds :type Float%20%28single-precision%29)))

(fn ConstructionScript
  (bind _returnvalue (Math|Random|RandomFloatinRange -3e+03 3e+03))
  (bind _end (Variables|Default|GetEnd))
  (Variables|Default|SetDir (Math|Vector|Normalize _end))
  (for _index (range 0 (Math|Float|Truncate (/ (Math|Vector|VectorLength _end) 1e+04)))
    (bind _output_get (Variables|Default|Setlocation (Math|Vector|MakeVector (.x (* _index 10000 (Variables|Default|GetDir))) (+ (.y (* _index 10000 (Variables|Default|GetDir))) _returnvalue) (+ (.z (* _index 10000 (Variables|Default|GetDir))) _returnvalue))))
    (AddComponent|AddStaticMeshComponent false (Math|Transform|MakeTransform _output_get "0, 0, 0" "1.000000,1.000000,1.000000"))
    (if (Math|Random|RandomBool)
      (AddComponent|AddChildActorComponent false (Math|Transform|MakeTransform _output_get "0, 0, 0" "1.000000,1.000000,1.000000")))))