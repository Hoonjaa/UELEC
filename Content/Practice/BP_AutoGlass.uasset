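; BP_AutoGlass is a procedurally laid strip of static mesh segments that destroys itself when its trigger box is overlapped.
; The construction script places meshes every 100 units along the FloorEnd direction, applying only roll and yaw from that direction.
; It then moves the Box one step past the last segment, so any overlap there removes the whole actor.
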(event OnComponentBeginOverlap(Box)
  (params (OverlappedComponent :type Primitive%20Component%20Object%20Reference) (OtherActor :type Actor%20Object%20Reference) (OtherComp :type Primitive%20Component%20Object%20Reference) (OtherBodyIndex :type Integer) (bFromSweep :type Boolean) (SweepResult :type Hit%20Result%20Structure%20%28by%20ref%29))
  (Actor|DestroyActor))

(event EventBeginPlay)

(event Collision|EventActorBeginOverlap
  (params (OtherActor :type Actor%20Object%20Reference)))

(event EventTick
  (params (DeltaSeconds :type Float%20%28single-precision%29)))

(fn ConstructionScript
  (bind _floorend (Variables|Default|GetFloorEnd))
  (Variables|Default|SetUnitDirection (Math|Vector|Normalize _floorend))
  (bind _output_get (Variables|Default|SetLast%20Index (Math|Float|Truncate (/ (Math|Vector|VectorLength _floorend) 1e+02))))
  (for _index (range 0 _output_get)
    (AddComponent|AddStaticMeshComponent false (Math|Transform|MakeTransform (* _index 100 (Variables|Default|GetUnitDirection)) (Math|Rotator|MakeRotator (.roll (Math|Conversions|RotationFromXVector (Variables|Default|GetUnitDirection))) 0.0 (.yaw (Math|Conversions|RotationFromXVector (Variables|Default|GetUnitDirection)))) "1.000000,1.000000,1.000000")))
  (Transformation|SetRelativeLocation (Variables|Default|GetBox) (* (+ (Variables|Default|GetLast%20Index) 1) 100 (Variables|Default|GetUnitDirection)) false false))